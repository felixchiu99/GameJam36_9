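; NPC character Blueprint that gets a random preference (Money, Usefulness or Looks) and can be directed toward a present.
; On BeginPlay it rolls the preference and creates a dynamic material instance, tinting the mesh with a color matching that preference.
; SetPresent writes the present's location to the AI Blackboard as a point of interest and raises the matching flag.
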(event `self.ReceiveBeginPlay`
  (bind _material (`self.Material`))
  (bind _mesh (`self.Mesh`))
  (`parent.ReceiveBeginPlay`)
  (set `self.Preference` (cast `ENpcPreference` (`KismetMathLibrary.Conv_IntToByte` (`KismetMathLibrary.RandomIntegerInRange` 1 3))))
  (bind _returnvalue (`PrimitiveComponent.CreateDynamicMaterialInstance` _mesh 0 (`PrimitiveComponent.GetMaterial` _mesh 0) "None"))
  (set `self.Material` _returnvalue)
  (switch `ENpcPreference` (`self.Preference`)
    (:`Money`
      (`MaterialInstanceDynamic.SetVectorParameterValue` _material "tint" (struct :`R` 1.0 :`G` 0.933874 :`A` 1.0)))
    (:`Usefulness`
      (`MaterialInstanceDynamic.SetVectorParameterValue` _material "tint" (struct :`G` 0.076538 :`B` 1.0 :`A` 1.0)))
    (:`Looks`
      (`MaterialInstanceDynamic.SetVectorParameterValue` _material "tint" (struct :`R` 1.0 :`B` 0.731755 :`A` 1.0))))
  (`PrimitiveComponent.SetMaterial` (`self.Mesh`) 0 (`self.Material`)))

(event `self.SetPresent`
  (params (present :type "PresentPawn Object Reference"))
  (bind _returnvalue (`AIBlueprintHelperLibrary.GetBlackboard` null))
  (`BlackboardComponent.SetValueAsVector` _returnvalue "PointOfInterest" (`self.K2_GetActorLocation` present))
  (`BlackboardComponent.SetValueAsBool` _returnvalue "bPointOfInterest" true))

(fn `UserConstructionScript`)